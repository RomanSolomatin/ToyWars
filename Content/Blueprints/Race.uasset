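; Race manager that tracks checkpoint progress and detects when the player has finished the course.
; On BeginPlay it gathers all RaceCheckPoint actors and polls them on a looping timer, showing only the one whose Order matches CurrentCheckpointIndex.
; When the index equals the checkpoint count, it prints a win message, stops polling and clears the InGameMenu's time-text timer.
; The index is advanced outside this Blueprint, and the Arrow-spawning logic is disconnected.
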(event `self.ReceiveBeginPlay`
  (bind _outactors (`GameplayStatics.GetAllActorsOfClass` "/Game/Blueprints/RaceCheckPoint.RaceCheckPoint_C"))
  (set `self.Checkpoints` _outactors)
  (`KismetSystemLibrary.K2_SetTimer` self "UpdateCheckpoints" 0.2 true))

(fn `UpdateCheckpoints`
  (if (== (`KismetArrayLibrary.Array_Length` (`self.Checkpoints`)) (`self.CurrentCheckpointIndex`))
    (`KismetSystemLibrary.PrintString` "Win Game")
    (`KismetSystemLibrary.K2_ClearTimer` self "UpdateCheckpoints")
    (bind _foundwidgets (`WidgetBlueprintLibrary.GetAllWidgetsOfClass` "/Game/Flying/UI/InGameMenu.InGameMenu_C"))
    (bind _asin_game_menu (cast `/Game/Flying/UI/InGameMenu` (`KismetArrayLibrary.Array_Get` _foundwidgets)))
    (`KismetSystemLibrary.K2_ClearTimer` _asin_game_menu "SetTimeText")
    (else
      (for _array_element (`self.Checkpoints`)
        (if (== (`/Game/Blueprints/RaceCheckPoint.Order` _array_element) (`self.CurrentCheckpointIndex`))
          (`SceneComponent.SetVisibility` _array_element true false)
          (else
            (`SceneComponent.SetVisibility` _array_element false false)))))))

(fn `UserConstructionScript`)