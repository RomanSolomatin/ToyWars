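; Race checkpoint actor that registers when a FlyShooterPawn flies through it and advances the race's progress.
; The Trigger's first overlap passes a one-shot gate before the pawn cast, setting Checked only if that actor is a FlyShooterPawn.
; Tick polls Checked, then once destroys a component, fires activation and playback feedback, and increments CurrentCheckpointIndex on the Race game mode.
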(event `self.ReceiveBeginPlay`)

(event `self.ReceiveActorBeginOverlap`
  (params (OtherActor :type "Actor Object Reference")))

(event `self.ReceiveTick`
  (params (DeltaSeconds :type "Float (single-precision)"))
  (if (`self.Checked`)
    (`/Engine/EditorBlueprintResources/StandardMacros.DoOnce` false
      (:`Completed`
        (`ActorComponent.K2_DestroyComponent`)
        (`ActorComponent.Activate` false)
        (`AudioComponent.Play` 0.0)
        (bind _asrace (cast `/Game/Blueprints/Race` (`GameplayStatics.GetGameMode`)))
        (set `/Game/Blueprints/Race.CurrentCheckpointIndex` (+ (`/Game/Blueprints/Race.CurrentCheckpointIndex` _asrace) 1) _asrace)))))

(event `self.Trigger.OnComponentBeginOverlap`
  (params (OtherActor :type "Actor Object Reference") (OtherComp :type "PrimitiveComponent Object Reference") (OtherBodyIndex :type Integer) (bFromSweep :type Boolean) (SweepResult :type "EngineTypes.HitResult Structure (by ref)"))
  (`/Engine/EditorBlueprintResources/StandardMacros.DoOnce` false
    (:`Completed`
      (cast `FlyShooterPawn` OtherActor)
      (set `self.Checked` true))))

(fn `UserConstructionScript`)